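; Weapon base Blueprint that fires shots through a BulletPenetration component.
; Fire shoots from the weapon mesh's muzzle socket along its forward vector, ignoring the weapon and its owner and crediting the first player controller as instigator.
; The component's hit damage event only prints the physical material name as debug output.
; A multi-shot loop and a random spread rotation are present but disconnected, so each Fire sends one straight shot.
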(event HitDamageEvent(BulletPenetration)
  (params (Hit :type Hit%20Result%20Structure) (Instigator :type Controller%20Object%20Reference) (Causer :type Actor%20Object%20Reference) (HitLocation :type Vector :default "0, 0, 0") (Damage :type Float%20%28single-precision%29) (Penetration :type Float%20%28single-precision%29) (Distance :type Float%20%28single-precision%29))
  (Development|PrintString (Utilities|GetDisplayName (.PhysMat (Collision|BreakHitResult Hit))) true true "(R=1.000000,G=0.038618,B=0.000000,A=1.000000)"))

(event Custom|Fire
  (bind _muzzlesocket (Variables|Default|GetMuzzleSocket))
  (bind _weaponmesh (Variables|Default|GetWeaponMesh))
  (bind _returnvalue (Transformation|GetSocketTransform _weaponmesh _muzzlesocket "RTS_World"))
  (bind (_location _rotation) (Math|Transform|BreakTransform _returnvalue))
  (Class|BulletPenetrationComponent|Shoot (Variables|Default|GetBulletPenetration) _location (* (Math|Vector|GetForwardVector _rotation) 1.5e+04) (Utilities|Array|MakeArray self (Components|GetOwner)) (Game|GetPlayerController 0)))

(fn ConstructionScript)