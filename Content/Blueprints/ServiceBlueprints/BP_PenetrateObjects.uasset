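; BP_PenetrateObjects is a service actor that labels a static mesh with the name of its physical material.
; The construction script and BeginPlay run the same logic, placing a text render just above the mesh bounds and sizing it from the box extent.
; The text comes from the physical material of the mesh's first material slot, or reads "No Material" when the mesh component is invalid.
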(event EventBeginPlay
  (bind _staticmesh (Variables|Default|GetStaticMesh))
  (bind _boxextent (Collision|GetComponentBounds _staticmesh))
  (Transformation|SetRelativeLocation (Variables|Default|GetTextRender) (Math|Vector|MakeVector 0.0 0.0 (+ (.z _boxextent) 2e+01)) false false)
  (Rendering|Components|TextRender|SetWorldSize (Variables|Default|GetTextRender) (.y _boxextent))
  (bind _staticmesh_2 (Variables|Default|GetStaticMesh)
    (:then
      (Rendering|Components|TextRender|SetText (Variables|Default|GetTextRender) (Utilities|Text|ToText(String) (Utilities|GetObjectName (Class|MaterialInterface|GetPhysicalMaterial (Rendering|Material|GetMaterial _staticmesh_2 0))))))
    (:else
      (Rendering|Components|TextRender|SetText (Variables|Default|GetTextRender) (Utilities|Text|MakeLiteralText "No Material")))))

(fn ConstructionScript
  (bind _staticmesh (Variables|Default|GetStaticMesh))
  (bind _boxextent (Collision|GetComponentBounds _staticmesh))
  (Transformation|SetRelativeLocation (Variables|Default|GetTextRender) (Math|Vector|MakeVector 0.0 0.0 (+ (.z _boxextent) 2e+01)) false false)
  (Rendering|Components|TextRender|SetWorldSize (Variables|Default|GetTextRender) (.y _boxextent))
  (bind _staticmesh_2 (Variables|Default|GetStaticMesh)
    (:then
      (Rendering|Components|TextRender|SetText (Variables|Default|GetTextRender) (Utilities|Text|ToText(String) (Utilities|GetObjectName (Class|MaterialInterface|GetPhysicalMaterial (Rendering|Material|GetMaterial _staticmesh_2 0))))))
    (:else
      (Rendering|Components|TextRender|SetText (Variables|Default|GetTextRender) (Utilities|Text|MakeLiteralText "No Material")))))