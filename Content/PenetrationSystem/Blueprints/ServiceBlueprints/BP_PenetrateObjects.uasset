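; BP_PenetrateObjects is a penetration-system actor that labels its static mesh with the name of the physical material from the mesh's first material slot.
; SetTextLocation traces against the mesh component from above its bounds down to the actor origin, then floats the text just over the hit.
; The text follows the actor's yaw at unit world scale.
; The update runs in both the construction script and BeginPlay.
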(event Custom|SetTextLocation
  (bind _returnvalue (Transformation|GetActorLocation))
  (bind _staticmeshcomponent (Variables|Debug|GetStaticMeshComponent)
    (:then
      (bind _hitlocation (Collision|LineTraceComponent (Variables|Debug|GetStaticMeshComponent) (+ _returnvalue (* (.z (.BoxExtent (Collision|GetComponentBounds _staticmeshcomponent))) (Math|Vector|VectorUp) 1.1)) _returnvalue true true false))
      (Transformation|SetWorldLocationAndRotation (Variables|Default|GetTextRender) (+ (* (Math|Vector|VectorUp) 1e+01) _hitlocation) (Math|Rotator|MakeRotator 0.0 0.0 (.yaw (Transformation|GetActorRotation))) false false)
      (Rendering|Components|TextRender|SetText (Variables|Default|GetTextRender) (Utilities|Text|ToText(String) (Utilities|GetObjectName (Class|MaterialInterface|GetPhysicalMaterial (Rendering|Material|GetMaterial (Variables|Debug|GetStaticMeshComponent) 0)))))
      (Transformation|SetWorldScale3D (Variables|Default|GetTextRender) "1.000000,1.000000,1.000000"))
    (:else)))

(event EventBeginPlay
  (CallFunction|SetTextLocation))

(fn ConstructionScript
  (CallFunction|SetTextLocation))