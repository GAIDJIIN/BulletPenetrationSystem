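; BP_PlayerCore is the player-controlled pawn in the PenetrationSystem, handling movement, look and weapon input.
; ChangeWeapon, run on BeginPlay and the X debug key, picks a class from the Weapon array, spawns it and snaps it to WeaponSpawn as CurrentWeapon.
; It does not destroy the previous weapon.
; Fire and the Z debug key call the current weapon's Fire and ToggleSpreadMode, leaving shooting logic to the weapon.
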(event EventBeginPlay
  (CallFunction|ChangeWeapon))

(event Input|ActionEvents|InputActionFire
  (params (Key :type Key%20Structure))
  (:Pressed
    (bind _currentweapon (Variables|Default|GetCurrentWeapon)
      (:then
        (Default|Fire _currentweapon))
      (:else))))

(event Input|AxisEvents|InputAxisMoveFB
  (params (AxisValue :type Float%20%28single-precision%29))
  (Pawn|Input|AddMovementInput (Transformation|GetActorForwardVector) AxisValue false))

(event Input|AxisEvents|InputAxisMoveLR
  (params (AxisValue :type Float%20%28single-precision%29))
  (Pawn|Input|AddMovementInput (Transformation|GetActorRightVector) AxisValue false))

(event Input|AxisEvents|InputAxisLookLR
  (params (AxisValue :type Float%20%28single-precision%29))
  (Pawn|Input|AddControllerYawInput AxisValue))

(event Input|AxisEvents|InputAxisLookUD
  (params (AxisValue :type Float%20%28single-precision%29))
  (Pawn|Input|AddControllerPitchInput AxisValue))

(event Input|KeyboardEvents|DebugKeyZ
  (params (Key :type Key%20Structure) (ActionValue :type Input%20Action%20Value%20Structure))
  (:Pressed
    (bind _currentweapon (Variables|Default|GetCurrentWeapon)
      (:then
        (Default|ToggleSpreadMode _currentweapon))
      (:else))))

(event Input|KeyboardEvents|DebugKeyX
  (params (Key :type Key%20Structure) (ActionValue :type Input%20Action%20Value%20Structure))
  (:Pressed
    (CallFunction|ChangeWeapon)))

(fn ConstructionScript)

(fn ChangeWeapon
  (bind _weapon (Variables|Default|GetWeapon))
  ;[1 1 1] Change Weapon or Spawn New
  (LocalVariables|SetLocalWeaponClass (select (or (Utilities|IsValid (Variables|Default|GetCurrentWeapon)) (== (Utilities|Array|FindItem _weapon (Utilities|GetClass (Variables|Default|GetCurrentWeapon))) (- (Utilities|Array|Length _weapon) 1))) (Utilities|Array|Get(acopy) (Variables|Default|GetWeapon)) (Utilities|Array|Get(acopy) _weapon (+ (Utilities|Array|FindItem _weapon (Utilities|GetClass (Variables|Default|GetCurrentWeapon))) 1))))
  (bind _returnvalue (Game|SpawnActorfromClass (LocalVariables|GetLocalWeaponClass) (Math|Transform|MakeTransform "0, 0, 0") "Undefined" 0 0))
  (Transformation|AttachComponentToComponent _returnvalue (Variables|Default|GetWeaponSpawn) "None" "SnapToTarget" "SnapToTarget" "SnapToTarget" true)
  (Variables|Default|SetCurrentWeapon _returnvalue))